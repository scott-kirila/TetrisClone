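; BP_SpawnManager is a Blueprint that, despite its name, only handles showing the game-over screen and contains no spawning logic.
; The DisplayGameOverScreen event creates a BP_GameOver widget for the stored PlayerController, adds it to the viewport, switches to UI-only input and shows the mouse cursor.
; EndPlay removes that widget if it is still valid.
; BeginPlay, Tick, overlap and the construction script are empty.
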(event EventBeginPlay)

(event Collision|EventActorBeginOverlap
  (params (OtherActor :type Actor%20Object%20Reference)))

(event EventTick
  (params (DeltaSeconds :type Float%20%28single-precision%29)))

(event EventDisplayGameOverScreen
  (bind _returnvalue (UserInterface|CreateWidget "/Game/Blueprints/UI/BP_GameOver.BP_GameOver_C" (Variables|Default|GetPlayerController)))
  (bind _output_get (Variables|Default|SetGameOverWidget _returnvalue))
  (UserInterface|Viewport|AddtoViewport _output_get 0)
  (Input|SetInputModeUIOnly (Variables|Default|GetPlayerController) (Variables|Default|GetGameOverWidget) "DoNotLock" false)
  (Variables|/Script/Engine.PlayerController|SetbShowMouseCursor (Variables|Default|GetPlayerController) true))

(event EventEndPlay
  (params (EndPlayReason :type EEndPlayReason%20Enum :default "Destroyed"))
  (bind _gameoverwidget (Variables|Default|GetGameOverWidget))
  (if (Utilities|IsValid _gameoverwidget)
    (Widget|RemovefromParent _gameoverwidget)))

(fn ConstructionScript)