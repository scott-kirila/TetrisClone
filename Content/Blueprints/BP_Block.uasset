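; BP_Block is a block actor that takes its color from the Piece that parents it.
; Both the construction script and BeginPlay cast the parent actor to Piece and apply that Piece's Color as material 0 on the static mesh.
; A failed cast prints an error, and BeginPlay first prints the current material's name for debugging.
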(event EventBeginPlay
  (Development|PrintString (Utilities|GetDisplayName (Rendering|Material|GetMaterial (Variables|Default|GetStaticMeshComponent) 0)))
  (bind _aspiece (Utilities|Casting|CastToPiece (Variables|Default|GetParentActor))
    (:then
      (Rendering|Material|SetMaterial (Variables|Default|GetStaticMeshComponent) 0 (Variables|/Script/TetrisClone.Piece|GetColor _aspiece)))
    (:CastFailed
      (Development|PrintString "Cast Failed!"))))

(event Collision|EventActorBeginOverlap
  (params (OtherActor :type Actor%20Object%20Reference)))

(event EventTick
  (params (DeltaSeconds :type Float%20%28single-precision%29)))

(fn ConstructionScript
  (bind _aspiece (Utilities|Casting|CastToPiece (Variables|Default|GetParentActor))
    (:then
      (Rendering|Material|SetMaterial (Variables|Default|GetStaticMeshComponent) 0 (Variables|/Script/TetrisClone.Piece|GetColor _aspiece)))
    (:CastFailed
      (Development|PrintString "Cast Failed!"))))